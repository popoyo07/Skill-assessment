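; Game instance that persists a gamma setting through an SGB_Save object in the SettingSlot save slot.
; On Init it loads that slot or creates a new save object, issuing a tonemapper gamma console command (spelled "r.TonemapperGama", no space) only for a new one.
; SaveSettings writes the slot first and assigns the new GamaValue only afterwards, so the written save holds the previous value.
; LoadSettings returns the cached value when the object is valid.
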(event Custom|LoadGame
  (bind _returnvalue (SaveGame|DoesSaveGameExist (Variables|Default|GetSettingSlot%20)))
  (if _returnvalue
    (bind _returnvalue_2 (SaveGame|LoadGamefromSlot (Variables|Default|GetSettingSlot%20)))
    (bind _assgb_save (Utilities|Casting|CastToSGB_Save _returnvalue_2))
    (Variables|Default|SetSGB_settomgs _assgb_save)
    (Development|PrintString "Load")
    (else
      (bind _returnvalue_3 (SaveGame|CreateSaveGameObject "/Game/Blue_Prints/SGB_Save.SGB_Save_C"))
      (bind _output_get (Variables|Default|SetSGB_settomgs _returnvalue_3))
      (Development|ExecuteConsoleCommand (Utilities|String|ToString(Text) (Utilities|Text|FormatText "r.TonemapperGama{x}" (Variables|/Game/Blue_Prints/SGB_Save.SGB_Save_C|GetGamaValue _output_get))) (Game|GetPlayerController 0)))))

(event Custom|SaveSettings
  (params (GamaValue :type Float%20%28double-precision%29))
  (bind _returnvalue (SaveGame|SaveGametoSlot (Variables|Default|GetSGB_settomgs) (Variables|Default|GetSettingSlot%20)))
  (if _returnvalue
    (Variables|/Game/Blue_Prints/SGB_Save.SGB_Save_C|SetGamaValue (Variables|Default|GetSGB_settomgs) GamaValue)
    (Development|PrintString "Settings Saved!!!")))

(event EventInit
  (CallFunction|LoadGame))

(fn LoadSettings
  (bind _sgb_settomgs (Variables|Default|GetSGB_settomgs)
    (:then
      (Development|PrintString "Settings Valid")
      (return (Variables|/Game/Blue_Prints/SGB_Save.SGB_Save_C|GetGamaValue _sgb_settomgs)))
    (:else)))