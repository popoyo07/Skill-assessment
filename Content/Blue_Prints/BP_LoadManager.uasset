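; BP_LoadManager is a level streaming actor that loads and unloads two map sections as the player passes through trigger volumes.
; Each overlap of BP_ThirdPersonCharacter with ManageSection1 or ManageSection2 toggles the matching soft-referenced level, tracked by a loaded flag per section.
; Loading and unloading are non-blocking, and loaded levels become visible immediately after loading.
; Only begin-overlap events drive the toggle.
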(event OnComponentBeginOverlap(ManageSection2)
  (params (OverlappedComponent :type Primitive%20Component%20Object%20Reference) (OtherActor :type Actor%20Object%20Reference) (OtherComp :type Primitive%20Component%20Object%20Reference) (OtherBodyIndex :type Integer) (bFromSweep :type Boolean) (SweepResult :type Hit%20Result%20Structure%20%28by%20ref%29))
  (Utilities|Casting|CastToBP_ThirdPersonCharacter OtherActor)
  (if (not (Variables|Default|GetLoadedSection2))
    (Class|GameplayStatics|LoadStreamLevelbySoftObjectPtr "/Game/SubLevels/SecondSection.SecondSection" true false)
    (Variables|Default|SetLoadedSection2 true)
    (else
      (Class|GameplayStatics|UnloadStreamLevelbySoftObjectPtr "/Game/SubLevels/SecondSection.SecondSection" false)
      (Variables|Default|SetLoadedSection2 false))))

(event OnComponentBeginOverlap(ManageSection1)
  (params (OverlappedComponent :type Primitive%20Component%20Object%20Reference) (OtherActor :type Actor%20Object%20Reference) (OtherComp :type Primitive%20Component%20Object%20Reference) (OtherBodyIndex :type Integer) (bFromSweep :type Boolean) (SweepResult :type Hit%20Result%20Structure%20%28by%20ref%29))
  (Utilities|Casting|CastToBP_ThirdPersonCharacter OtherActor)
  (if (not (Variables|Default|GetLoadedSection1))
    (Class|GameplayStatics|LoadStreamLevelbySoftObjectPtr "/Game/SubLevels/FirstSection.FirstSection" true false)
    (Variables|Default|SetLoadedSection1 true)
    (else
      (Class|GameplayStatics|UnloadStreamLevelbySoftObjectPtr "/Game/SubLevels/FirstSection.FirstSection" false)
      (Variables|Default|SetLoadedSection1 false))))

(event EventBeginPlay)

(event Collision|EventActorBeginOverlap
  (params (OtherActor :type Actor%20Object%20Reference)))

(event EventTick
  (params (DeltaSeconds :type Float%20%28single-precision%29)))

(fn ConstructionScript)