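; BP_Ball is an interactable pickup that hands a ball to the third-person character.
; Overlapping its Sphere1 component stores the BP_ThirdPersonCharacter reference and shows a widget, which hides again when the overlap ends.
; OnInteraction sets the stored character's ThisStaticMesh to the GizmoSphereHandle mesh, then destroys the ball actor.
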(event OnComponentBeginOverlap(Sphere1)
  (params (OverlappedComponent :type Primitive%20Component%20Object%20Reference) (OtherActor :type Actor%20Object%20Reference) (OtherComp :type Primitive%20Component%20Object%20Reference) (OtherBodyIndex :type Integer) (bFromSweep :type Boolean) (SweepResult :type Hit%20Result%20Structure%20%28by%20ref%29))
  (bind _asbp_third_person_character (Utilities|Casting|CastToBP_ThirdPersonCharacter OtherActor))
  (Variables|Default|SetThird%20person%20character _asbp_third_person_character)
  (Rendering|SetVisibility (Variables|Default|GetWidget) true false))

(event OnComponentEndOverlap(Sphere1)
  (params (OverlappedComponent :type Primitive%20Component%20Object%20Reference) (OtherActor :type Actor%20Object%20Reference) (OtherComp :type Primitive%20Component%20Object%20Reference) (OtherBodyIndex :type Integer))
  (Utilities|Casting|CastToBP_ThirdPersonCharacter OtherActor)
  (Rendering|SetVisibility (Variables|Default|GetWidget) false false))

(event EventOnInteraction
  (Components|StaticMesh|SetStaticMesh (Variables|/Game/ThirdPerson/Blueprints/BP_ThirdPersonCharacter.BP_ThirdPersonCharacter_C|GetThis%20static%20mesh%20 (Variables|Default|GetThird%20person%20character)) "/Engine/InteractiveToolsFramework/Meshes/GizmoSphereHandle.GizmoSphereHandle")
  (Actor|DestroyActor))

(fn ConstructionScript)